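; Trigger actor that raises the BP_Jeremy character's progression stats when it walks into one of three collision zones.
; Separate overlap events increment CharacterLevel, CharacterXP or Currency by one, ignoring any other actor through a cast.
; Each change is saved immediately, with level and XP going through SaveCharacterData and currency through SaveCurrency.
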(event OnComponentBeginOverlap(IncreaseLevelCollision)
  (params (OverlappedComponent :type Primitive%20Component%20Object%20Reference) (OtherActor :type Actor%20Object%20Reference) (OtherComp :type Primitive%20Component%20Object%20Reference) (OtherBodyIndex :type Integer) (bFromSweep :type Boolean) (SweepResult :type Hit%20Result%20Structure%20%28by%20ref%29))
  (bind _asbp_jeremy (Utilities|Casting|CastToBP_Jeremy OtherActor))
  (Math|Float|IncrementFloat (Variables|/Script/StickySituation.PlayerCharacterBase|GetCharacterLevel _asbp_jeremy)
    (:%20%20
      (Class|PlayerCharacterBase|SaveCharacterData _asbp_jeremy))))

(event OnComponentBeginOverlap(IncreaseXPCollision)
  (params (OverlappedComponent :type Primitive%20Component%20Object%20Reference) (OtherActor :type Actor%20Object%20Reference) (OtherComp :type Primitive%20Component%20Object%20Reference) (OtherBodyIndex :type Integer) (bFromSweep :type Boolean) (SweepResult :type Hit%20Result%20Structure%20%28by%20ref%29))
  (bind _asbp_jeremy (Utilities|Casting|CastToBP_Jeremy OtherActor))
  (Math|Float|IncrementFloat (Variables|/Script/StickySituation.PlayerCharacterBase|GetCharacterXP _asbp_jeremy)
    (:%20%20
      (Class|PlayerCharacterBase|SaveCharacterData _asbp_jeremy))))

(event OnComponentBeginOverlap(IncreaseCurrencyCollision)
  (params (OverlappedComponent :type Primitive%20Component%20Object%20Reference) (OtherActor :type Actor%20Object%20Reference) (OtherComp :type Primitive%20Component%20Object%20Reference) (OtherBodyIndex :type Integer) (bFromSweep :type Boolean) (SweepResult :type Hit%20Result%20Structure%20%28by%20ref%29))
  (bind _asbp_jeremy (Utilities|Casting|CastToBP_Jeremy OtherActor))
  (Math|Float|IncrementFloat (Variables|/Script/StickySituation.PlayerCharacterBase|GetCurrency _asbp_jeremy)
    (:%20%20
      (Class|PlayerCharacterBase|SaveCurrency _asbp_jeremy))))

(fn ConstructionScript)