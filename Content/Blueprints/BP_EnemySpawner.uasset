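; Enemy spawner actor that periodically spawns random enemy types at its spawn point once StartSpawning is called.
; StartSpawning sets a looping two-second timer, guarded against duplicates by a handle check, that fires SpawnEnemy.
; SpawnEnemy skips the tick while a BP_BaseEnemy still overlaps the sphere, so the previous one can clear the spawn point.
; Otherwise it spawns a random class from EnemyTypes and notifies the game mode via EnemySpawnedMessage.
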(event Custom|SpawnEnemy
  (if (not (Utilities|Array|IsValidIndex (Collision|GetOverlappingActors (Variables|Default|GetSphere) "/Game/Blueprints/Characters/Enemies/BP_BaseEnemy.BP_BaseEnemy_C" :!class /Script/Engine.PrimitiveComponent)))
    (bind _enemytype (CallFunction|SelectRandomEnemy))
    (Game|SpawnActorfromClass _enemytype (Math|Transform|MakeTransform (Transformation|GetWorldLocation (Variables|Default|GetspawnPoint)) "0, 0, 0" "1.000000,1.000000,1.000000") "Undefined" "MultiplyWithRoot" 0 0)
    (Class|BPIWaveSystem|EnemySpawned(Message) (Game|GetGameMode))))

(event EventStartSpawning
  (if (not (Utilities|Time|IsValidTimerHandle (Variables|Default|GetSpawnerTimer)))
    (bind _returnvalue (Utilities|Time|SetTimerbyEvent (delegate Custom|SpawnEnemy) 2.0 true))
    (Variables|Default|SetSpawnerTimer _returnvalue)))

(fn ConstructionScript)

(fn SelectRandomEnemy
  (bind _output_get (Variables|Default|SetcurrentEnemy (.OutItem (Utilities|Array|Random (Variables|Default|GetEnemyTypes)))))
  (return _output_get))