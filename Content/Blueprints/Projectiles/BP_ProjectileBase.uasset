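; Base projectile Blueprint that explodes on hitting an actor and deals direct-hit damage to enemies.
; Its component hit event spawns a Niagara effect and sound at its location, and derives a ragdoll direction pointing toward the hit actor.
; Actors tagged "enemy" receive damage and that direction through DirectHitDamageMessage.
; The projectile destroys itself after any valid actor hit, enemy or not.
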(event OnComponentHit(Projectile)
  (params (HitComponent :type Primitive%20Component%20Object%20Reference) (OtherActor :type Actor%20Object%20Reference) (OtherComp :type Primitive%20Component%20Object%20Reference) (NormalImpulse :type Vector :default "0, 0, 0") (Hit :type Hit%20Result%20Structure%20%28by%20ref%29))
  (bind _hitactor (Collision|BreakHitResult Hit))
  (Utilities|IsValid _hitactor
    (:Is%20Valid
      (Variables|Default|SetHitActor _hitactor)
      (Variables|Default|SetRagdollDirection (Math|Vector|GetForwardVector (Math|Rotator|FindLookatRotation (Transformation|GetActorLocation) (Transformation|GetActorLocation _hitactor))))
      (Niagara|SpawnSystematLocation (Variables|Default|GetSystem%20Template) (Transformation|GetActorLocation))
      (Audio|PlaySoundatLocation (Variables|Default|GetExplosionSound) (Transformation|GetActorLocation) "0, 0, 0" 1.0 1.0 0.0 0 0 0 0)
      (Utilities|IsValid (Variables|Default|GetHitActor)
        (:Is%20Valid
          (if (Actor|ActorHasTag (Variables|Default|GetHitActor) "enemy")
            (Class|BPIDamage|DirectHitDamage(Message) (Variables|Default|GetHitActor) (Variables|Default|GetHitDamage) (Variables|Default|GetRagdollDirection))
            (Actor|DestroyActor)
            (else
              (Actor|DestroyActor))))))))

(fn ConstructionScript)