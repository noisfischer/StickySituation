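; Knockout projectile that stuns actors tagged as enemy, both on impact and in an area when it is destroyed.
; A hit on the Projectile component sends StunMessage to the struck enemy.
; On destruction it spawns a Niagara goo effect, then runs a zero-length sphere trace on the Visibility channel to send StunMessage to nearby enemies.
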(event OnComponentHit(Projectile)
  (params (HitComponent :type Primitive%20Component%20Object%20Reference) (OtherActor :type Actor%20Object%20Reference) (OtherComp :type Primitive%20Component%20Object%20Reference) (NormalImpulse :type Vector :default "0, 0, 0") (Hit :type Hit%20Result%20Structure%20%28by%20ref%29))
  (if (Actor|ActorHasTag OtherActor "enemy")
    (Class|BPIDamage|Stun(Message) OtherActor)))

(event EventDestroyed
  (bind _returnvalue (Transformation|GetActorLocation))
  (Niagara|SpawnSystematLocation "/Game/PArticles/NS_KnockoutGoo.NS_KnockoutGoo" (Transformation|GetActorLocation))
  (bind (_outhits _returnvalue_2) (Collision|MultiSphereTraceByChannel _returnvalue _returnvalue 3e+02 "TraceTypeQuery1" false 0 "None" true "(R=0.202219,G=1.000000,B=0.000000,A=1.000000)" "(R=1.000000,G=0.000000,B=0.059195,A=1.000000)" 0.5))
  (if _returnvalue_2
    (for _array_element _outhits
      (if (Actor|ActorHasTag (.HitActor (Collision|BreakHitResult _array_element)) "enemy")
        (Class|BPIDamage|Stun(Message) (.HitActor (Collision|BreakHitResult _array_element)))))))

(fn ConstructionScript
  (|CallParentFunction))