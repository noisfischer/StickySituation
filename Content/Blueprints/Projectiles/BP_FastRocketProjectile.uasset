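; Fast rocket projectile Blueprint that explodes with area damage against enemies whenever it is destroyed.
; On Destroyed, it spawns a red hit Niagara effect and runs a stationary multi-sphere trace on the Visibility channel at its location.
; Each valid hit actor tagged "enemy" receives a blast-radius damage message with a ragdoll direction pointing away from the explosion.
; Movement and collision are not defined in this graph.
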(event EventDestroyed
  (bind _returnvalue (Transformation|GetActorLocation))
  (Niagara|SpawnSystematLocation "/Game/PArticles/NS_HitRed.NS_HitRed" (Transformation|GetActorLocation))
  (bind (_outhits _returnvalue_2) (Collision|MultiSphereTraceByChannel _returnvalue _returnvalue 4e+02 "TraceTypeQuery1" false 0 "None" true "(R=0.202219,G=1.000000,B=0.000000,A=1.000000)" "(R=1.000000,G=0.000000,B=0.059195,A=1.000000)" 0.5))
  (if _returnvalue_2
    (for _array_element _outhits
      (Utilities|IsValid (.HitActor (Collision|BreakHitResult _array_element))
        (:Is%20Valid
          (if (Actor|ActorHasTag (.HitActor (Collision|BreakHitResult _array_element)) "enemy")
            (Class|BPIDamage|BlastRadiusDamage(Message) (.HitActor (Collision|BreakHitResult _array_element)) 1e+01 (Math|Vector|GetForwardVector (Math|Rotator|FindLookatRotation (Transformation|GetActorLocation) (Transformation|GetActorLocation (.HitActor (Collision|BreakHitResult _array_element))))))))))))

(fn ConstructionScript
  (|CallParentFunction))