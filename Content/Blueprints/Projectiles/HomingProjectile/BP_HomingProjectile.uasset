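; Homing projectile that seeks an enemy and deals radial blast damage when destroyed.
; The first "enemy"-tagged actor overlapping HomingTracking becomes the ProjectileMovement homing target, then that detection component is destroyed.
; On destruction it spawns a green hit effect and sphere-traces for enemies, recording them in EnemiesDamaged.
; It messages them damage with an outward ragdoll direction, and sends EnemiesRemaining messages to the player character and game mode.
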(event OnComponentBeginOverlap(HomingTracking)
  (params (OverlappedComponent :type Primitive%20Component%20Object%20Reference) (OtherActor :type Actor%20Object%20Reference) (OtherComp :type Primitive%20Component%20Object%20Reference) (OtherBodyIndex :type Integer) (bFromSweep :type Boolean) (SweepResult :type Hit%20Result%20Structure%20%28by%20ref%29))
  ;[1 1 1] Select Target
  (if (Actor|ActorHasTag OtherActor "enemy")
    (bind _output_get (Variables|Default|SetEnemyTarget OtherActor))
    (Variables|/Script/Engine.ProjectileMovementComponent|SetHomingTargetComponent (Variables|Default|GetProjectileMovement) (Variables|/Script/Engine.Actor|GetRootComponent _output_get))
    (Components|DestroyComponent (Variables|Default|GetHomingTracking))))

(event EventBeginPlay
  (|CallParentFunction))

(event EventDestroyed
  (bind _returnvalue (Transformation|GetActorLocation))
  (Niagara|SpawnSystematLocation "/Game/PArticles/NS_HitGreen.NS_HitGreen" (Transformation|GetActorLocation))
  ;[1 1 1] Radial Blast
  (bind (_outhits _returnvalue_2) (Collision|MultiSphereTraceByChannel _returnvalue _returnvalue 5e+02 "TraceTypeQuery1" false 0 "None"))
  (if _returnvalue_2
    (for _array_element _outhits
      (Utilities|IsValid (.HitActor (Collision|BreakHitResult _array_element))
        (:Is%20Valid
          (if (Actor|ActorHasTag (.HitActor (Collision|BreakHitResult _array_element)) "enemy")
            (bind _array_element_2 (Utilities|Array|ForEachLoopwithBreak (Variables|Default|GetEnemiesDamaged) :!label _label)
              (:LoopBody
                (if (== _array_element_2 (.HitActor (Collision|BreakHitResult _array_element)))
                  (goto _label Break)))
              (:Completed
                (Utilities|Array|Add (Variables|Default|GetEnemiesDamaged) (.HitActor (Collision|BreakHitResult _array_element)))
                (Class|BPIDamage|BlastRadiusDamage(Message) (.HitActor (Collision|BreakHitResult _array_element)) 1e+01 (Math|Vector|GetForwardVector (Math|Rotator|FindLookatRotation (Transformation|GetActorLocation) (Transformation|GetActorLocation (.HitActor (Collision|BreakHitResult _array_element))))))
                (Class|BPIWaveSystem|EnemiesRemaining(Message) (Game|GetPlayerCharacter 0))
                (Class|BPIWaveSystem|EnemiesRemaining(Message) (Game|GetGameMode))))))))))

(fn ConstructionScript
  (|CallParentFunction))