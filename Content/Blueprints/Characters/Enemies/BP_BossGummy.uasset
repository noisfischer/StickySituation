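; BP_BossGummy is a boss enemy whose destruction ends the encounter and can trigger the player's win.
; On Destroyed, it checks the third-person player's Dead flag, and only if the player lives does it clear its Alive flag and send a win message.
; Either way, it tells the game mode to stop spawning and messages every actor tagged "enemy" to despawn.
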(event EventDestroyed
  (bind _asbp_third_person_character (Utilities|Casting|CastToBP_ThirdPersonCharacter (Game|GetPlayerCharacter 0)))
  (if (Variables|/Game/Blueprints/Characters/BP_ThirdPersonCharacter.BP_ThirdPersonCharacter_C|Getdead _asbp_third_person_character)
    (Class|BPIWaveSystem|StopSpawning(Message) (Game|GetGameMode))
    (bind _outactors (Actor|GetAllActorswithTag "enemy"))
    (for _array_element _outactors
      (Class|BPIWaveSystem|Despawn(Message) _array_element))
    (else
      (Variables|Default|Setalive false)
      (Class|BPIWaveSystem|Win(Message) (Game|GetPlayerCharacter 0))
      (Class|BPIWaveSystem|StopSpawning(Message) (Game|GetGameMode))
      (bind _outactors_2 (Actor|GetAllActorswithTag "enemy"))
      (for _array_element_2 _outactors_2
        (Class|BPIWaveSystem|Despawn(Message) _array_element_2)))))

(fn ConstructionScript
  (|CallParentFunction))