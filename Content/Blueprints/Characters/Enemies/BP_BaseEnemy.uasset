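; Base enemy character that endlessly re-issues AI MoveTo toward the player and self-destructs on contact, dealing damage.
; Direct, blast and acid damage events share SubtractHealth; lethal damage plays effects, notifies player and game mode, then destroys it.
; Stun and melee events temporarily freeze non-boss enemies, swapping material and adding a tag that disables contact damage.
; Destruction randomly drops health pickups; ragdoll impulse code is disconnected.
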(event OnComponentHit(CapsuleComponent)
  (params (HitComponent :type Primitive%20Component%20Object%20Reference) (OtherActor :type Actor%20Object%20Reference) (OtherComp :type Primitive%20Component%20Object%20Reference) (NormalImpulse :type Vector :default "0, 0, 0") (Hit :type Hit%20Result%20Structure%20%28by%20ref%29))
  (Utilities|IsValid OtherActor
    (:Is%20Valid
      (if (Math|Boolean|ANDBoolean (Actor|ActorHasTag OtherActor "player") (not (Actor|ActorHasTag self "stunned")) (not (Variables|Default|GetenemyDead?)))
        (Class|BPIDamage|DirectHitDamage(Message) OtherActor (Variables|Default|GetDamage) "0, 0, 0")
        (Niagara|SpawnSystematLocation (Variables|Default|GetDeathParticles) (Transformation|GetActorLocation))
        (Audio|SpawnSoundatLocation (Variables|Default|GetDeathSound) (Transformation|GetActorLocation) "0, 0, 0" 1.0 1.0 0.0 0 0)
        (Class|BPIWaveSystem|EnemiesRemaining(Message) (Game|GetGameMode))
        (Variables|Default|SetenemyDead? true)
        (Actor|DestroyActor)))))

(event Custom|MoveToPlayer
  (bind _returnvalue (Game|GetPlayerCharacter 0))
  (AI|AIMoveTo self (Transformation|GetActorLocation _returnvalue) _returnvalue 5.0 false
    (:OnSuccess
      _)
    (:OnFail
      _))
  (CallFunction|MovetoPlayer))

(event EventAcidDamage
  (params (Damage :type Float%20%28double-precision%29))
  (if (not (Variables|Default|GetenemyDead?))
    (Audio|PlaySoundatLocation "/Game/Audio/SFX/Cue/Acid_Damage_Cue.Acid_Damage_Cue" (Transformation|GetActorLocation) "0, 0, 0" 1.0 1.0 0.0 0 0 0 0)
    (bind _healthfullydepleted_ (CallFunction|SubtractHealth Damage))
    (if _healthfullydepleted_
      (Variables|Default|SetenemyDead? true)
      (Niagara|SpawnSystematLocation (Variables|Default|GetDeathParticles) (Transformation|GetActorLocation))
      (Class|BPIDamage|KilledEnemy(Message) (Game|GetPlayerCharacter 0))
      (Class|BPIWaveSystem|EnemiesRemaining(Message) (Game|GetGameMode))
      (Actor|DestroyActor))))

(event EventStun
  (if (not (or (Variables|Default|Getstunned) (Variables|Default|GetisBoss)))
    (Audio|PlaySoundatLocation "/Game/Audio/SFX/Cue/Melee_Hit_Cue.Melee_Hit_Cue" (Transformation|GetActorLocation) "0, 0, 0" 1.0 1.0 0.0 0 0 0 0)
    (Niagara|SpawnSystematLocation (Variables|Default|GetDeathParticles) (Transformation|GetActorLocation))
    (Variables|/Script/Engine.CharacterMovementComponent|SetMaxWalkSpeed (Variables|Character|GetCharacterMovement) 0.0)
    (Utilities|Array|Add (Variables|Actor|GetTags) "stunned")
    (Rendering|Material|SetMaterial (Variables|Character|GetMesh) (Variables|Default|GetElement%20Index) "/Game/Materials/GummieBears_Inst_Knockout.GummieBears_Inst_Knockout")
    (Variables|Default|Setstunned true)
    (Utilities|FlowControl|Delay 5.0)
    (Variables|/Script/Engine.CharacterMovementComponent|SetMaxWalkSpeed (Variables|Character|GetCharacterMovement) (Variables|Default|GetnormalSpeed))
    (Utilities|Array|RemoveItem (Variables|Actor|GetTags) "stunned")
    (Rendering|Material|SetMaterial (Variables|Character|GetMesh) (Variables|Default|GetElement%20Index) (Variables|Default|GetOriginalMaterial))
    (Variables|Default|Setstunned false)))

(event EventBeginPlay
  (bind _returnvalue (Game|GetPlayerCharacter 0))
  (Variables|Default|SetOriginalMaterial (Rendering|Material|GetMaterial (Variables|Character|GetMesh) 0))
  (AI|AIMoveTo self (Transformation|GetActorLocation _returnvalue) _returnvalue 5.0 false
    (:OnSuccess
      _)
    (:OnFail
      _))
  (CallFunction|MovetoPlayer))

(event EventDirectHitDamage
  (params (Damage :type Float%20%28double-precision%29) (HitDirection :type Vector :default "0, 0, 0"))
  (if (not (Variables|Default|GetenemyDead?))
    (Audio|PlaySoundatLocation "/Game/Audio/SFX/Cue/Melee_Hit_Cue.Melee_Hit_Cue" (Transformation|GetActorLocation) "0, 0, 0" 1.0 1.0 0.0 0 0 0 0)
    (bind _healthfullydepleted_ (CallFunction|SubtractHealth Damage))
    (if _healthfullydepleted_
      (Utilities|FlowControl|DoOnce false
        (:Completed
          (CallFunction|EnemyKilled HitDirection))))))

(event EventBlastRadiusDamage
  (params (Damage :type Float%20%28double-precision%29) (RagdollDirection :type Vector :default "0, 0, 0"))
  (if (not (Variables|Default|GetenemyDead?))
    (bind _healthfullydepleted_ (CallFunction|SubtractHealth Damage))
    (if _healthfullydepleted_
      (Utilities|FlowControl|DoOnce false
        (:Completed
          (CallFunction|EnemyKilled RagdollDirection))))))

(event EventMeleeDamage
  (if (not (or (Variables|Default|Getstunned) (Variables|Default|GetisBoss)))
    (Audio|PlaySoundatLocation "/Game/Audio/SFX/Cue/Melee_Hit_Cue.Melee_Hit_Cue" (Transformation|GetActorLocation) "0, 0, 0" 1.0 1.0 0.0 0 0 0 0)
    (Niagara|SpawnSystematLocation (Variables|Default|GetDeathParticles) (Transformation|GetActorLocation))
    (Variables|/Script/Engine.CharacterMovementComponent|SetMaxWalkSpeed (Variables|Character|GetCharacterMovement) 0.0)
    (Utilities|Array|Add (Variables|Actor|GetTags) "stunned")
    (Rendering|Material|SetMaterial (Variables|Character|GetMesh) (Variables|Default|GetElement%20Index) "/Game/Materials/GummieBears_Inst_Knockout.GummieBears_Inst_Knockout")
    (Variables|Default|Setstunned true)
    (Utilities|FlowControl|Delay 5.0)
    (Variables|/Script/Engine.CharacterMovementComponent|SetMaxWalkSpeed (Variables|Character|GetCharacterMovement) (Variables|Default|GetnormalSpeed))
    (Utilities|Array|RemoveItem (Variables|Actor|GetTags) "stunned")
    (Rendering|Material|SetMaterial (Variables|Character|GetMesh) (Variables|Default|GetElement%20Index) (Variables|Default|GetOriginalMaterial))
    (Variables|Default|Setstunned false)))

(event EventDespawn
  (Niagara|SpawnSystematLocation (Variables|Default|GetDeathParticles) (Transformation|GetActorLocation))
  (Audio|PlaySoundatLocation "/Game/Audio/SFX/Cue/EnemyDeathCue.EnemyDeathCue" (Transformation|GetActorLocation) "0, 0, 0" 1.0 1.0 0.0 0 0 0 0)
  (Actor|DestroyActor))

(event EventDestroyed
  (if (== 1 (Math|Random|RandomIntegerinRange 1 20))
    (Game|SpawnActorfromClass "/Game/Blueprints/BP_HealthPickup.BP_HealthPickup_C" (Math|Transform|MakeTransform (Transformation|GetActorLocation) "0, 0, 0" "1.000000,1.000000,1.000000") "Undefined" "MultiplyWithRoot" 0 0)))

(fn ConstructionScript)

(fn EnemyKilled
  (params (RagdollDirection :type Vector))
  (Niagara|SpawnSystematLocation (Variables|Default|GetDeathParticles) (Transformation|GetActorLocation))
  (Variables|Default|SetenemyDead? true)
  (Audio|PlaySoundatLocation "/Game/Audio/SFX/Cue/EnemyDeathCue.EnemyDeathCue" (Transformation|GetActorLocation) "0, 0, 0" 1.0 1.0 0.0 0 0 0 0)
  (Class|BPIDamage|KilledEnemy(Message) (Game|GetPlayerCharacter 0))
  (Class|BPIWaveSystem|EnemiesRemaining(Message) (Game|GetGameMode))
  (Actor|DestroyActor))

(fn SubtractHealth
  (params (DamageTaken :type Float%20%28double-precision%29))
  (bind _output_get (Variables|Default|SetcurrentHealth (- (Variables|Default|GetcurrentHealth) DamageTaken)))
  (return (<= _output_get 0.0)))