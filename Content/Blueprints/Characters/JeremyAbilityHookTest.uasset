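; Test projectile actor for Jeremy's grapple hook ability that flies toward a point along the player's aim direction.
; On BeginPlay it traces out to the grapple range, snaps the endpoint to any hit and sets the ProjectileMovement velocity toward it.
; It destroys itself on reaching the endpoint after a missed trace, or when its mesh hits anything except the player, recording its height first.
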(event OnComponentHit(StaticMesh)
  (params (HitComponent :type Primitive%20Component%20Object%20Reference) (OtherActor :type Actor%20Object%20Reference) (OtherComp :type Primitive%20Component%20Object%20Reference) (NormalImpulse :type Vector :default "0, 0, 0") (Hit :type Hit%20Result%20Structure%20%28by%20ref%29))
  (if (not (== (Game|GetPlayerCharacter 0) OtherActor))
    (Variables|Default|SetHeight (.z (Transformation|GetActorLocation)))
    (Actor|DestroyActor)))

(event EventBeginPlay
  (Variables|Default|SetEndLocation (+ (Variables|Default|GetStartLocation) (* (Variables|Default|GetPlayerDirection) (Variables|Default|GetGrappleRange))))
  (bind (_outhit _returnvalue) (Collision|LineTraceByChannel (Variables|Default|GetStartLocation) (Variables|Default|GetEndLocation) "TraceTypeQuery1" false 0 "ForDuration" true "(R=1.000000,G=0.000000,B=0.000000,A=1.000000)" "(R=0.000000,G=1.000000,B=0.000000,A=1.000000)" 1.0))
  (if _returnvalue
    (Variables|Default|SetbHit true)
    (Variables|Default|SetEndLocation (.Location (Collision|BreakHitResult _outhit)))
    (else
      (Variables|Default|SetbHit false)))
  (bind _output_get (Variables|Default|SetDirection (Math|Vector|Normalize (- (Variables|Default|GetEndLocation) (Variables|Default|GetStartLocation)))))
  (Variables|/Script/Engine.MovementComponent|SetVelocity (Variables|Default|GetProjectileMovement) (* _output_get (Variables|Default|GetSpeed))))

(event EventTick
  (params (DeltaSeconds :type Float%20%28single-precision%29))
  (if (not (Variables|Default|GetbHit))
    (if (Utilities|Operators|EqualEqual (Transformation|GetActorLocation) (Variables|Default|GetEndLocation) 1e+01)
      (Actor|DestroyActor))))

(fn ConstructionScript)