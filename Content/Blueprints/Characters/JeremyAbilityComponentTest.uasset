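; Test ability Blueprint for Jeremy that provides a grappling hook on right mouse button.
; The press spawns a JeremyAbilityHookTest near the player, aimed along the follow camera's forward vector.
; When the hook is destroyed after a hit, its OnDestroyed event launches the player toward the hook's end point.
; The launch overrides velocity, taking horizontal speed from the scaled direction and vertical speed from the difference in absolute heights.
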(event Custom|LaunchCharacter
  (params (DestroyedActor :type Actor%20Object%20Reference))
  (bind _playerref (Variables|Default|GetPlayerRef))
  (bind _currentgrapple (Variables|Default|GetCurrentGrapple))
  (bind _returnvalue (Transformation|GetActorLocation _playerref))
  (bind _height (Variables|/Game/Blueprints/Characters/JeremyAbilityHookTest.JeremyAbilityHookTest_C|GetHeight _currentgrapple))
  (bind _returnvalue_2 (Math|Float|Absolute(Float) (.z _returnvalue)))
  (bind _returnvalue_3 (Math|Float|Absolute(Float) _height))
  (bind _returnvalue_4 (- _returnvalue_3 _returnvalue_2))
  (if (Variables|/Game/Blueprints/Characters/JeremyAbilityHookTest.JeremyAbilityHookTest_C|GetbHit (stale Input|MouseEvents|RightMouseButton _output_get))
    (Variables|Default|SetHeightMultiplier (Math|Float|Absolute(Float) _returnvalue_4))
    (if (< _returnvalue_4 0.0)
      (Character|LaunchCharacter (Variables|Default|GetPlayerRef) (Math|Vector|MakeVector (.x (* (Math|Vector|Normalize (- (Variables|/Game/Blueprints/Characters/JeremyAbilityHookTest.JeremyAbilityHookTest_C|GetEndLocation (stale Input|MouseEvents|RightMouseButton _output_get)) (Transformation|GetActorLocation (Game|GetPlayerCharacter 0)))) 2.5e+03)) (.y (* (Math|Vector|Normalize (- (Variables|/Game/Blueprints/Characters/JeremyAbilityHookTest.JeremyAbilityHookTest_C|GetEndLocation (stale Input|MouseEvents|RightMouseButton _output_get)) (Transformation|GetActorLocation (Game|GetPlayerCharacter 0)))) 2.5e+03)) (* (Variables|Default|GetHeightMultiplier) -2.0)) true true)
      (else
        (Character|LaunchCharacter (Variables|Default|GetPlayerRef) (Math|Vector|MakeVector (.x (* (Math|Vector|Normalize (- (Variables|/Game/Blueprints/Characters/JeremyAbilityHookTest.JeremyAbilityHookTest_C|GetEndLocation (stale Input|MouseEvents|RightMouseButton _output_get)) (Transformation|GetActorLocation (Game|GetPlayerCharacter 0)))) 2.5e+03)) (.y (* (Math|Vector|Normalize (- (Variables|/Game/Blueprints/Characters/JeremyAbilityHookTest.JeremyAbilityHookTest_C|GetEndLocation (stale Input|MouseEvents|RightMouseButton _output_get)) (Transformation|GetActorLocation (Game|GetPlayerCharacter 0)))) 2.5e+03)) (* (Variables|Default|GetHeightMultiplier) 2.0)) true true)))))

(event EventBeginPlay
  (bind _asbp_jeremy (Utilities|Casting|CastToBP_Jeremy (Game|GetPlayerCharacter 0)))
  (Variables|Default|SetPlayerRef _asbp_jeremy))

(event Input|MouseEvents|RightMouseButton
  (params (Key :type Key%20Structure :default "None"))
  (bind _playerref (Variables|Default|GetPlayerRef))
  (bind _returnvalue (Transformation|GetActorLocation _playerref))
  (bind _followcamera (Variables|/Script/StickySituation.PlayerCharacterBase|GetFollowCamera _playerref))
  (bind _returnvalue_2 (Transformation|GetWorldRotation _followcamera))
  (bind _returnvalue_3 (+ _returnvalue "100.000000,100.000000,0.000000"))
  (:Pressed
    (bind _returnvalue_4 (Game|SpawnActorfromClass "/Game/Blueprints/Characters/JeremyAbilityHookTest.JeremyAbilityHookTest_C" (Math|Transform|MakeTransform _returnvalue_3 _returnvalue_2 "1.000000,1.000000,1.000000") "Undefined" "MultiplyWithRoot" 0 _returnvalue_3 (Math|Vector|GetForwardVector _returnvalue_2) 0))
    (bind _output_get (Variables|Default|SetCurrentGrapple _returnvalue_4))
    (Game|BindEventtoOnDestroyed _output_get (delegate Custom|LaunchCharacter))))