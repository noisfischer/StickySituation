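; BP_ConveyorBelt_P2P is a point-to-point conveyor actor that moves from its placed position toward an end location and loops back.
; BeginPlay records the start location and applies Speed to the ProjectileMovement component as initial and max speed.
; Tick teleport-resets it to the start, without sweep, once X or Y exceeds EndLocation, so the check only catches travel toward positive X or Y.
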(event EventBeginPlay
  (bind _projectilemovement (Variables|Default|GetProjectileMovement))
  (bind _output_get (Variables|/Script/Engine.ProjectileMovementComponent|SetInitialSpeed _projectilemovement (Variables|Movement|Getspeed)))
  (Variables|/Script/Engine.ProjectileMovementComponent|SetMaxSpeed _projectilemovement _output_get)
  (bind _output_get_2 (Variables|Movement|SetstartLocation (Transformation|GetActorLocation)))
  (Variables|Movement|SetendLocation (Variables|Movement|GetendLocation))
  (Transformation|SetActorLocation _output_get_2 false false))

(event EventTick
  (params (DeltaSeconds :type Float%20%28single-precision%29))
  (bind _returnvalue (Transformation|GetActorLocation))
  (bind _endlocation (Variables|Movement|GetendLocation))
  (bind (_x _y) (Math|Vector|BreakVector _endlocation))
  (bind (_x_2 _y_2) (Math|Vector|BreakVector _returnvalue))
  (if (or (> _x_2 _x) (> _y_2 _y))
    (Transformation|SetActorLocation (stale EventBeginPlay _output_get_2) false false)))

(fn ConstructionScript)