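; Game mode that runs endless enemy waves, each 20 enemies larger than the last, with music and player notifications.
; StartWave triggers every BP_EnemySpawner found at BeginPlay, and spawn events pause them by clearing their timers once EnemyLimit is reached.
; Death events count down the wave and can resume spawning.
; At zero, EndWave stops spawners, despawns "enemy"-tagged actors and fades music before the next wave starts after a delay.
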(event EventBeginPlay
  (bind _outactors (Actor|GetAllActorsOfClass "/Game/Blueprints/BP_EnemySpawner.BP_EnemySpawner_C"))
  (Variables|Default|SetSpawners _outactors)
  (CallFunction|StartWave) ; Start spawning
)

(event EventEnemiesRemaining
  (params (enemiesLeft :type Integer))
  ;[0 0 0] On Enemy Death
  (bind _result (Math|Integer|DecrementInt (Variables|Default|GetenemiesLeft))
    (:%20%20
      (Class|BPIWaveSystem|EnemiesRemaining(Message) (Game|GetPlayerCharacter 0) _result)
      (if (<= _result 0)
        (CallFunction|EndWave)
        (Utilities|FlowControl|Delay 5.0)
        (Audio|PlaySound2D "/Game/Audio/SFX/Suzy/Cue/StartVoice_Cue.StartVoice_Cue" 1.0 1.0 0.0 0 0)
        (CallFunction|StartWave)
        (else
          (bind _result_2 (Math|Integer|DecrementInt (Variables|Default|GetcurrentEnemyPool))
            (:%20%20
              (if (and (Variables|Default|GetspawningPaused) (< _result_2 (Variables|Default|GetenemiesLeft)))
                (CallFunction|ResumeSpawning)))))))))

(event EventResetWaves
  (bind _output_get (Variables|Default|SetmaxEnemies 0))
  (Variables|Default|SetenemiesLeft _output_get)
  (CallFunction|StartWave))

(event EventStopSpawning
  (CallFunction|PauseSpawning))

(event EventEnemySpawned
  ;[0 0 0] When enemy is spawned, check if enemy limit has been met
  (bind _result (Math|Integer|IncrementInt (Variables|Default|GetcurrentEnemyPool))
    (:%20%20
      (if (>= _result (Variables|Default|GetenemyLimit))
        (CallFunction|PauseSpawning)
        (Variables|Default|SetspawningPaused true)))))

(event EventClearMusic
  (bind _music (Variables|Default|GetMusic)
    (:then
      (Audio|Components|Audio|FadeOut _music 1.0 0.0 "Linear" :!class /Script/Engine.AudioComponent))
    (:else)))

(fn ConstructionScript)

(fn StartWave
  (bind _output_get (Variables|Default|SetmaxEnemies (+ (Variables|Default|GetmaxEnemies) 20)))
  (bind _output_get_2 (Variables|Default|SetenemiesLeft _output_get))
  (Class|BPIWaveSystem|NextWave(Message) (Game|GetPlayerCharacter 0) _output_get_2)
  (Variables|Default|SetenemiesKilled 0)
  (Variables|Default|SetcurrentEnemyPool 0)
  (for _array_element (Variables|Default|GetSpawners)
    (Class|BPIWaveSystem|StartSpawning(Message) _array_element))
  (bind _returnvalue (Audio|SpawnSound2D "/Game/Audio/Music/MusicRandomizer.MusicRandomizer" 1.0 1.0 0.0 0))
  (bind _output_get_3 (Variables|Default|SetMusic _returnvalue))
  (Audio|Components|Audio|FadeIn (Variables|Default|GetMusic) 1.0 1.0 0.0 "Linear" :!class /Script/Engine.AudioComponent))

(fn EndWave
  (bind _music (Variables|Default|GetMusic))
  (for _array_element (Variables|Default|GetSpawners)
    (Utilities|Time|ClearandInvalidateTimerbyHandle (Variables|/Game/Blueprints/BP_EnemySpawner.BP_EnemySpawner_C|GetSpawnerTimer _array_element)))
  (bind _outactors (Actor|GetAllActorswithTag "enemy"))
  (for _array_element_2 _outactors
    (Utilities|IsValid _array_element_2
      (:Is%20Valid
        (Class|BPIWaveSystem|Despawn(Message) _array_element_2))))
  (Audio|PlaySound2D "/Game/Audio/SFX/Suzy/Wave/just_like_jeremy_2_riverside.just_like_jeremy_2_riverside" 0.5 1.0 0.0 0 0)
  (Utilities|IsValid _music
    (:Is%20Valid
      (Audio|Components|Audio|FadeOut _music 1.0 0.0 "Linear" :!class /Script/Engine.AudioComponent))))

(fn EnterTransition)

(fn PauseSpawning
  (for _array_element (Variables|Default|GetSpawners)
    (Utilities|Time|ClearandInvalidateTimerbyHandle (Variables|/Game/Blueprints/BP_EnemySpawner.BP_EnemySpawner_C|GetSpawnerTimer _array_element))))

(fn ResumeSpawning
  (for _array_element (Variables|Default|GetSpawners)
    (Class|BPIWaveSystem|StartSpawning(Message) _array_element)))